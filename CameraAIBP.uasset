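; Security camera actor that detects BP_RU74_Character through overlap and raises an alarm.
; On overlap, a Camera-channel line trace to the character confirms line of sight before detection counts.
; Detection swaps materials, plays a sound, calls AlertAllGuards on every MrAlertBP and spawns a StairLockBP at a fixed location for a timed lockdown.
; Ending any overlap clears the detection flag and switches the materials to their undetected look.
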(event `self.ReceiveActorBeginOverlap`
  (params (OtherActor :type "Actor Object Reference"))
  ;[1 1 1] On Detect
  (bind _returnvalue (`GameplayStatics.GetActorOfClass` "/Game/BP_RU74_Character.BP_RU74_Character_C"))
  (bind _outhit (`KismetSystemLibrary.LineTraceSingle` (`self.K2_GetActorLocation`) (`self.K2_GetActorLocation` _returnvalue) "TraceTypeQuery2"))
  (if (== (`.HitActor` (`GameplayStatics.BreakHitResult` _outhit)) _returnvalue)
    (set `self.HitSomething?` (== OtherActor _returnvalue))
    (if (`self.HitSomething?`) :!label _label
      (`PrimitiveComponent.SetMaterial` (`self.Detect`) 0 "/Engine/EngineMaterials/EditorBrushMaterial.EditorBrushMaterial")
      (`GameplayStatics.PlaySoundAtLocation` "/Engine/EditorSounds/Notifications/CompileFailed.CompileFailed" (0.0 0.0 0.0) (struct) 1.0 1.0 0.0 null null null null)
      (`PrimitiveComponent.SetMaterial` (`self.StaticMesh1`) 0 "/Engine/EditorLandscapeResources/LayerVisMaterial.LayerVisMaterial")
      (bind _outactors (`GameplayStatics.GetAllActorsOfClass` "/Game/MrAlertBP.MrAlertBP_C"))
      (`/Game/MrAlertBP.AlertAllGuards` _outactors)
      (bind _returnvalue_2 (`|SpawnActorFromClass` "/Game/StairLockBP.StairLockBP_C" (`KismetMathLibrary.MakeTransform` (-2482.0 1452.0 727.0)) "Undefined" "MultiplyWithRoot" null null))
      (`KismetSystemLibrary.Delay` 30.0)
      (`self.K2_DestroyActor` _returnvalue_2)
      (else
        (`PrimitiveComponent.SetMaterial` (`self.Detect`) 0 "/Engine/VREditor/UI/ArrowMaterial.ArrowMaterial")
        (`PrimitiveComponent.SetMaterial` (`self.StaticMesh1`) 0 "/Engine/VREditor/UI/ArrowMaterial.ArrowMaterial")))))

(event `self.ReceiveActorEndOverlap`
  (params (OtherActor :type "Actor Object Reference"))
  ;[1 1 1] On Detect
  (set `self.HitSomething?` false)
  (goto _label))

(fn `UserConstructionScript`)