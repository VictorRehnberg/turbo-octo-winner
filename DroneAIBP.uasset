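; DroneAIBP is a drone AI character that takes damage and can be destroyed.
; AnyDamage subtracts damage from Health, but destroys the actor only when Health is already zero or below as a hit arrives.
; UpdateWalkSpeed sets the movement component's max walk speed.
; ChangeLightColor swaps the mesh's material at index 1 between two materials based on the TriggerLight flag.
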(event `self.ReceiveTick`
  (params (DeltaSeconds :type "Float (single-precision)")))

(event `self.ReceiveAnyDamage`
  (params (Damage :type "Float (single-precision)") (DamageType :type "DamageType Object Reference") (InstigatedBy :type "Controller Object Reference") (DamageCauser :type "Actor Object Reference"))
  ;[1 1 1] Take Damage
  (if (<= (`self.Health`) 0.0)
    (`self.K2_DestroyActor`)
    (else
      (set `self.Health` (- (`self.Health`) Damage)))))

(fn `ChangeLightColor`
  (bind _mesh (`self.Mesh`))
  (if (`self.TriggerLight?`)
    (`PrimitiveComponent.SetMaterial` _mesh 1 "/Engine/EditorLandscapeResources/LayerVisMaterial.LayerVisMaterial")
    (else
      (`PrimitiveComponent.SetMaterial` _mesh 1 "/Engine/VREditor/UI/ArrowMaterial.ArrowMaterial"))))

(fn `UpdateWalkSpeed`
  (params (NewWalkSpeed :type "Float (double-precision)"))
  (set `CharacterMovementComponent.MaxWalkSpeed` NewWalkSpeed (`self.CharacterMovement`)))

(fn `UserConstructionScript`)